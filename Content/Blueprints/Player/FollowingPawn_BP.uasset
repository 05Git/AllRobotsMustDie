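; FollowingPawn_BP is a player-side pawn that automatically attacks an enemy touching its hitbox.
; Hitbox overlap events store the BasicEnemy_BP and set an overlap flag, which Tick polls.
; Each attack deals fixed damage, plays an explosion sound and briefly toggles AttackSprite, with delays and an IsAttacking flag forming the cooldown.
; Only the last enemy to enter is tracked, and any enemy leaving clears the overlap flag.
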(event `self.ReceiveBeginPlay`
  (`SceneComponent.ToggleVisibility` (`self.AttackSprite`) false))

(event `self.ReceiveTick`
  (params (DeltaSeconds :type "Float (single-precision)"))
  (bind _returnvalue (`self.IsOverlappingEnemy`))
  (if _returnvalue
    (bind _returnvalue_2 (`self.IsAttacking`))
    (if (not _returnvalue_2)
      (`BasicEnemy.ReceiveDamage` (`self.OverlappedEnemy`) 10.0)
      (`SceneComponent.ToggleVisibility` (`self.AttackSprite`) false)
      (`self.SetIsAttacking` true)
      (`self.PlayExplosionSound`)
      (`KismetSystemLibrary.Delay` 0.5)
      (`SceneComponent.ToggleVisibility` (`self.AttackSprite`) false)
      (`KismetSystemLibrary.Delay` 1.5)
      (`self.SetIsAttacking` false))))

(event `self.Hitbox.OnComponentBeginOverlap`
  (params (OverlappedComponent :type "PrimitiveComponent Object Reference") (OtherActor :type "Actor Object Reference") (OtherComp :type "PrimitiveComponent Object Reference") (OtherBodyIndex :type Integer) (bFromSweep :type Boolean) (SweepResult :type "HitResult Structure (by ref)"))
  (bind _asbasic_enemy_bp (cast `/Game/Blueprints/Enemies/BasicEnemy/BasicEnemy_BP` OtherActor))
  (set `self.OverlappedEnemy` _asbasic_enemy_bp)
  (`self.SetIsOverlappingEnemy` true))

(event `self.Hitbox.OnComponentEndOverlap`
  (params (OverlappedComponent :type "PrimitiveComponent Object Reference") (OtherActor :type "Actor Object Reference") (OtherComp :type "PrimitiveComponent Object Reference") (OtherBodyIndex :type Integer))
  (cast `/Game/Blueprints/Enemies/BasicEnemy/BasicEnemy_BP` OtherActor)
  (`self.SetIsOverlappingEnemy` false))

(fn `UserConstructionScript`)