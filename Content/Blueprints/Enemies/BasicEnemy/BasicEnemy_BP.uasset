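; Basic enemy that repeatedly damages the player character while the player stands inside its hitbox.
; Hitbox begin and end overlap events set an overlapping flag, which Tick polls alongside an attacking flag.
; Each attack applies fixed damage, toggles the attack sprite and plays an electric sound.
; Delays toggle the sprite back, then clear the attacking flag, forming a cooldown between hits.
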(event `self.ReceiveBeginPlay`
  (`SceneComponent.ToggleVisibility` (`self.AttackSprite`) false))

(event `self.ReceiveTick`
  (params (DeltaSeconds :type "Float (single-precision)"))
  (bind _returnvalue (`self.GetIsOverlapping`))
  (if _returnvalue
    (bind _returnvalue_2 (`self.GetIsAttacking`))
    (if (not _returnvalue_2)
      (bind _asplayer_char_bp (cast `/Game/Blueprints/Player/PlayerChar_BP` (`GameplayStatics.GetPlayerCharacter` 0)))
      (`PlayerChar.ReceiveDamage` _asplayer_char_bp 20.0)
      (`SceneComponent.ToggleVisibility` (`self.AttackSprite`) false)
      (`self.PlayElectricSound`)
      (`self.SetIsAttacking` true)
      (`KismetSystemLibrary.Delay` 0.5)
      (`SceneComponent.ToggleVisibility` (`self.AttackSprite`) false)
      (`KismetSystemLibrary.Delay` 1.0)
      (`self.SetIsAttacking` false))))

(event `self.Hitbox.OnComponentBeginOverlap`
  (params (OverlappedComponent :type "PrimitiveComponent Object Reference") (OtherActor :type "Actor Object Reference") (OtherComp :type "PrimitiveComponent Object Reference") (OtherBodyIndex :type Integer) (bFromSweep :type Boolean) (SweepResult :type "HitResult Structure (by ref)"))
  (cast `/Game/Blueprints/Player/PlayerChar_BP` OtherActor)
  (`self.SetIsOverlapping` true))

(event `self.Hitbox.OnComponentEndOverlap`
  (params (OverlappedComponent :type "PrimitiveComponent Object Reference") (OtherActor :type "Actor Object Reference") (OtherComp :type "PrimitiveComponent Object Reference") (OtherBodyIndex :type Integer))
  (cast `/Game/Blueprints/Player/PlayerChar_BP` OtherActor)
  (`self.SetIsOverlapping` false))

(fn `UserConstructionScript`)